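; Player controller Blueprint for the Neuron plugin that plays back BVH motion capture files.
; On BeginPlay it initializes the Neuron controller from a reference skeleton BVH file, or with default init plus a hard-coded hips bone offset.
; Successful init starts playback with configurable looping, reference bone, displacement and line format, storing the result in NeuronConnected.
; The Pause input action toggles playback pause.
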(event `self.ReceiveActorBeginOverlap`
  (params (OtherActor :type "Actor Object Reference")))

(event `self.ReceiveTick`
  (params (DeltaSeconds :type "Float (single-precision)")))

(event `/Game/NeuronPlugin/Blueprints/BP_NetworkNeuronController.ReceiveBeginPlay`
  ;[1 1 1] On BeginPlay Init Neuron Controller and play BVH File
  (if (`self.InitWithBVHReferenceFile`)
    (bind _returnvalue (`PerceptionNeuronBPLibrary.NeuronInitFile` self (`self.ReferenceSkeletonFileName`)))
    (if _returnvalue
      (bind _returnvalue_2 (`PerceptionNeuronBPLibrary.NeuronPlay` self (`self.BVHFileName`) (`self.PlayEndless`) (`self.EnableReferenceBone`) (`self.Enable Displacement`) (`self.Motion Line Format`) :!label _label))
      (set `self.NeuronConnected` _returnvalue_2))
    (else
      (bind _returnvalue_3 (`PerceptionNeuronBPLibrary.NeuronInit` self))
      (if _returnvalue_3
        (bind _returnvalue_4 (`PerceptionNeuronBPLibrary.NeuronBoneSetOffset` self 0 0.0 95.32)) ; Set Hips Bone Offset
        (if _returnvalue_4
          (goto _label))))))

(event `InputAction|Pause`
  (params (Key :type "Key Structure" :default "AnyKey"))
  ;[1 1 1] On Pause Hit toggle playing BVH File
  (:`Pressed`
    (bind _output_get (set `self.PauseToggle` (not (`self.PauseToggle`))))
    (`PerceptionNeuronBPLibrary.NeuronPause` self _output_get)))

(fn `UserConstructionScript`)