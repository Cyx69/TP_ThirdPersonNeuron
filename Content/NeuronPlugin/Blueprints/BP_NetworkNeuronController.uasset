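; Neuron plugin controller actor that connects to a motion data stream over the network.
; On BeginPlay it initializes from a reference skeleton BVH file, then connects using the configured host, port, reference bone, displacement and line format settings.
; A Reconnect event disconnects and connects again, with a blocker flag guarding against re-entry.
; Each connection attempt stores its result in NeuronConnected.
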(event `self.ReceiveActorBeginOverlap`
  (params (OtherActor :type "Actor Object Reference")))

(event `self.ReceiveTick`
  (params (DeltaSeconds :type "Float (single-precision)")))

(event `self.ReceiveBeginPlay`
  ;[1 1 1] On BeginPlay Init Neuron Controller and connect
  (bind _returnvalue (`PerceptionNeuronBPLibrary.NeuronInit` self (`self.ReferenceSkeletonFileName`)))
  (if _returnvalue
    (bind _returnvalue_2 (`PerceptionNeuronBPLibrary.NeuronConnect` self (`self.HostName`) (`self.Port`) (`self.EnableReferenceBone`) (`self.Enable Displacement`) (`self.Motion Line Format`)))
    (set `self.NeuronConnected` _returnvalue_2)))

(event `Reconnect_Event`
  ;[1 1 1] Reconnect Event
  (if (not (`self.ReconnectBlocker`))
    (set `self.ReconnectBlocker` true)
    (`PerceptionNeuronBPLibrary.NeuronDisconnect` self)
    (set `self.NeuronConnected` false)
    (bind _returnvalue (`PerceptionNeuronBPLibrary.NeuronConnect` self (`self.HostName`) (`self.Port`) (`self.EnableReferenceBone`) (`self.Enable Displacement`) (`self.Motion Line Format`)))
    (set `self.NeuronConnected` _returnvalue)
    (set `self.ReconnectBlocker` false)))

(fn `UserConstructionScript`)